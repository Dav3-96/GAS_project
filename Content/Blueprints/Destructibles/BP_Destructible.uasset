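; BP_Destructible is a destructible actor with GAS-based health that reacts to damage and is destroyed when its health runs out.
; On BeginPlay it applies GE_InitHealthSet to its own AbilitySystemComponent, setting max health through a SetByCaller tag.
; OnHealthChanged briefly rotates the static mesh and back as a hit shake while health is above zero, and destroys the actor otherwise.
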(event `self.ReceiveBeginPlay`
  (set `self.GE_Spec` (`AbilitySystemComponent.MakeOutgoingSpec` :`self` (`self.AbilitySystemComponent`) :`GameplayEffectClass` "/Game/Blueprints/GAS/Effects/GE_InitHealthSet.GE_InitHealthSet_C"))
  (bind _returnvalue (`AbilitySystemBlueprintLibrary.AssignTagSetByCallerMagnitude` (`self.GE_Spec`) (struct :`TagName` "HealthSet.Init.MaxHealth") 20.0))
  (`AbilitySystemComponent.BP_ApplyGameplayEffectSpecToSelf` (`self.AbilitySystemComponent`) _returnvalue))

(event `DMGShake`
  (`SceneComponent.K2_AddLocalRotation` (`self.StaticMesh`) (struct :`Yaw` 5.0) false true)
  (`KismetSystemLibrary.Delay` 0.05)
  (`SceneComponent.K2_AddLocalRotation` (`self.StaticMesh`) (struct :`Yaw` -5.0) false true))

(event `self.OnHealthChanged`
  (params (OldValue :type "Float (single-precision)") (NewValue :type "Float (single-precision)"))
  (if (> NewValue 0.0)
    (`self.DMGShake`)
    (else
      (`self.K2_DestroyActor`))))

(fn `UserConstructionScript`)