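; Gameplay Ability that fires a pistol by spawning a BP_PistolBullet for the third-person character avatar.
; On activation it casts the avatar, commits the ability, spawns the bullet and immediately ends.
; The spawn point is the mesh location nudged along the actor's forward vector and raised vertically, using actor rotation.
; The character owns the bullet, which always spawns, adjusting for collision if possible.
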(event `self.K2_ActivateAbility`
  (bind _character (`self.Character`))
  (bind _returnvalue (`Actor.K2_GetActorRotation` _character))
  (bind (_returnvalue_x _returnvalue_y _returnvalue_z) (`KismetMathLibrary.BreakVector` (+ (`SceneComponent.K2_GetComponentLocation` (`Character.Mesh` _character)) (`KismetMathLibrary.Conv_RotatorToVector` _returnvalue))))
  (bind _asbp_third_person_character (cast `/Game/Blueprints/Player/BP_ThirdPersonCharacter` (`self.GetAvatarActorFromActorInfo`)))
  (set `self.Character` _asbp_third_person_character)
  (`self.K2_CommitAbility`)
  (`|SpawnActorFromClass` "/Game/Blueprints/Weapons/Pistols/Example/BP_PistolBullet.BP_PistolBullet_C" (`KismetMathLibrary.MakeTransform` (`KismetMathLibrary.MakeVector` _returnvalue_x _returnvalue_y (+ _returnvalue_z 100.0)) _returnvalue) "AdjustIfPossibleButAlwaysSpawn" "MultiplyWithRoot" _character null)
  (`self.K2_EndAbility`))