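; Gameplay ability for the pistol's alternate fire, which shoots a quick three-round burst of BP_PistolBullet.
; On activation it caches the avatar as BP_ThirdPersonCharacter, commits without checking the result, then spawns bullets separated by short delays before ending.
; Each shot spawns just forward of and above the mesh's location, facing along the actor's rotation, with the character as owner.
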(event `self.K2_ActivateAbility`
  (bind _asbp_third_person_character (cast `/Game/Blueprints/Player/BP_ThirdPersonCharacter` (`self.GetAvatarActorFromActorInfo`)))
  (set `self.Character` _asbp_third_person_character)
  (`self.K2_CommitAbility`)
  (`self.SpawnProjectile`)
  (`KismetSystemLibrary.Delay` 0.05)
  (`self.SpawnProjectile`)
  (`KismetSystemLibrary.Delay` 0.05)
  (`self.SpawnProjectile`)
  (`self.K2_EndAbility`))

(fn `SpawnProjectile`
  (bind _character (`self.Character`))
  (bind _returnvalue (`Actor.K2_GetActorRotation` _character))
  (bind (_returnvalue_x _returnvalue_y _returnvalue_z) (`KismetMathLibrary.BreakVector` (+ (`SceneComponent.K2_GetComponentLocation` (`Character.Mesh` _character)) (`KismetMathLibrary.Conv_RotatorToVector` _returnvalue))))
  (`|SpawnActorFromClass` "/Game/Blueprints/Weapons/Pistols/Example/BP_PistolBullet.BP_PistolBullet_C" (`KismetMathLibrary.MakeTransform` (`KismetMathLibrary.MakeVector` _returnvalue_x _returnvalue_y (+ _returnvalue_z 100.0)) _returnvalue) "AdjustIfPossibleButAlwaysSpawn" "MultiplyWithRoot" _character null))