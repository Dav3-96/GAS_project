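; Gameplay ability that gives BP_ThirdPersonCharacter a short dash in the direction of its last movement input.
; On activation it commits the ability, then launches the avatar with the scaled input vector, added to its current velocity.
; After a brief delay it stops movement immediately and ends the ability, while a leftover AddMovementInput node stays unconnected.
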(event `self.K2_ActivateAbility`
  (bind _asbp_third_person_character (cast `/Game/Blueprints/Player/BP_ThirdPersonCharacter` (`self.GetAvatarActorFromActorInfo`)))
  (set `self.Character` _asbp_third_person_character)
  (`self.K2_CommitAbility`)
  (`Character.LaunchCharacter` (`self.Character`) (* (`Pawn.GetLastMovementInputVector` (`self.Character`)) 2000.0) false false)
  (`KismetSystemLibrary.Delay` 0.1)
  (`MovementComponent.StopMovementImmediately` (`Character.CharacterMovement` (`self.Character`)))
  (`self.K2_EndAbility`))